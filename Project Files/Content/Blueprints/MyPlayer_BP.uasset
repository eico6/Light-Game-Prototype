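; Player character with a HUD overlay, world-axis movement, jumping, mouse aiming and a flashlight.
; Each tick it turns toward the mouse ray's intersection with a horizontal plane at its height and sizes the flashlight's radius and cone from FlashLightCollider's scale.
; Takedamage lowers Health and destroys the actor at zero; Escape opens the main menu.
; Charged-shot and power-up timer logic is present but disconnected.
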(event `self.ReceiveBeginPlay`
  (bind _returnvalue (`|CreateWidget` "/Game/Blueprints/Widgets/WidgetBP_HUDOverlay.WidgetBP_HUDOverlay_C" (`GameplayStatics.GetPlayerController` 0)))
  (`UserWidget.AddToViewport` _returnvalue 0)
  (`ActorComponent.Activate` (`self.Camera1`) false)
  (`WidgetBlueprintLibrary.SetInputMode_GameOnly` (`GameplayStatics.GetPlayerController` 0))
  (`GameplayStatics.SetViewportMouseCaptureMode` "CapturePermanently_IncludingInitialMouseDown"))

(event `self.ReceiveTick`
  (params (DeltaSeconds :type "Float (single-precision)"))
  (bind (_returnvalue_x _returnvalue_y) (`KismetMathLibrary.BreakVector` (`SceneComponent.K2_GetComponentScale` (`self.FlashLightCollider`))))
  (`self.LookAtMouse`)
  (`LocalLightComponent.SetAttenuationRadius` (`self.Flashlight`) (* _returnvalue_y 170.0))
  (`SpotLightComponent.SetOuterConeAngle` (`self.Flashlight`) (* _returnvalue_y 5.0)))

(event `Key|Escape`
  (params (Key :type "Key Structure"))
  (:`Pressed`
    (`GameplayStatics.OpenLevel` "MainMenu")))

(event `InputAction|Shoot`
  (params (Key :type "Key Structure"))
  ;[1 1 1] Shoot enemy
)

(event `InputAxis|MoveForward`
  (params (AxisValue :type "Float (single-precision)"))
  ;[1 1 1] WASD and JUMP
  (`self.AddMovementInput` (1.0 0.0 0.0) AxisValue))

(event `InputAxis|MoveRight`
  (params (AxisValue :type "Float (single-precision)"))
  ;[1 1 1] WASD and JUMP
  (`self.AddMovementInput` (0.0 1.0 0.0) AxisValue))

(event `InputAction|Jump`
  (params (Key :type "Key Structure"))
  ;[1 1 1] WASD and JUMP
  (:`Pressed`
    (`self.Jump`))
  (:`Released`
    (`self.StopJumping`)))

(event `Take damage`
  (bind _health (`self.Health`))
  ;[1 1 1] Take Damage
  (set `self.Health` (- _health (`self.Damage Taken`)))
  (if (<= _health 0)
    (`KismetSystemLibrary.PrintString` "You died")
    (`self.K2_DestroyActor`)
    (else
      (`KismetSystemLibrary.PrintString` (`KismetStringLibrary.Conv_IntToString` (`self.Health`))))))

(fn `LookAtMouse`
  (bind _returnvalue (`self.K2_GetActorLocation`))
  (bind (_worldlocation _worlddirection) (`PlayerController.DeprojectMousePositionToWorld` (`GameplayStatics.GetPlayerController` 0)))
  (bind (_intersectionpoint _pointfound) (`self.GetRayAndPlaneIntersectionPoint` _worldlocation _worlddirection 50000.0 _returnvalue (0.0 0.0 1.0)))
  ;[1 1 1] Rotate player to look at where the mouse is
  (if _pointfound
    (`self.K2_SetActorRotation` (`KismetMathLibrary.FindLookAtRotation` _returnvalue _intersectionpoint))))

(fn `UserConstructionScript`)