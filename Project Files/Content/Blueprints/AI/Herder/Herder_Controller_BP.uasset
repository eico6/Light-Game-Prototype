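; AI controller for the Herder enemy that runs its behavior tree and keeps the blackboard supplied with state.
; On begin play it starts Herder_BT and stores the player character as PlayerObj.
; Every tick it copies the player's left and right point locations, plus the Herder pawn's stage and priority flags, into blackboard keys for the tree to read.
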(event `self.ReceiveBeginPlay`
  (`self.RunBehaviorTree` "/Game/Blueprints/AI/Herder/Herder_BT.Herder_BT")
  (`BlackboardComponent.SetValueAsObject` (`AIBlueprintHelperLibrary.GetBlackboard` null) "PlayerObj" (`GameplayStatics.GetPlayerCharacter` 0)))

(event `self.ReceiveTick`
  (params (DeltaSeconds :type "Float (single-precision)"))
  ;[1 1 1] Update variables in BlackBoard every frame for reference to AI
  (bind _asmy_player_bp (cast `/Game/Blueprints/MyPlayer_BP` (`GameplayStatics.GetPlayerCharacter` 0)))
  (set `self.RefToLeftLocation` (`MyPlayer.LeftPointLocation` _asmy_player_bp))
  (set `self.RefToRightLocation` (`MyPlayer.RightPointLocation` _asmy_player_bp))
  (`BlackboardComponent.SetValueAsVector` (`AIBlueprintHelperLibrary.GetBlackboard` null) "LeftLocation" (`self.RefToLeftLocation`))
  (`BlackboardComponent.SetValueAsVector` (`AIBlueprintHelperLibrary.GetBlackboard` null) "RightLocation" (`self.RefToRightLocation`))
  (bind _asherder_bp (cast `/Game/Blueprints/AI/Herder/Herder_BP` (`self.K2_GetPawn`)))
  (set `self.PrioritizeLeft` (`Herder.bPrioritizeLeft` _asherder_bp))
  (set `self.StageOneComplete` (`Herder.bStageOneComplete` _asherder_bp))
  (set `self.PrioritizePlayer` (`Herder.bPrioritizePlayer` _asherder_bp))
  (`BlackboardComponent.SetValueAsBool` (`AIBlueprintHelperLibrary.GetBlackboard` null) "PrioritizeLeft" (`self.PrioritizeLeft`))
  (`BlackboardComponent.SetValueAsBool` (`AIBlueprintHelperLibrary.GetBlackboard` null) "StageOneComplete" (`self.StageOneComplete`))
  (`BlackboardComponent.SetValueAsBool` (`AIBlueprintHelperLibrary.GetBlackboard` null) "PrioritizePlayer" (`self.PrioritizePlayer`)))

(fn `UserConstructionScript`)