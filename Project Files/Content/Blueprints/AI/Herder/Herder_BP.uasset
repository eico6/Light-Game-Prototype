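; Herder_BP is the AI Herder actor, which can keep itself turned toward the player and tracks a stage-completion flag.
; Each Tick, when RotateTowardsPlayer is set, it snaps to a yaw-only look-at rotation toward player character 0, leaving pitch and roll at zero.
; EnableStageTwo, noted as called from the MoveToPoint task in Herder_BT, sets StageOneComplete to true.
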(event `self.ReceiveTick`
  (params (DeltaSeconds :type "Float (single-precision)"))
  ;[1 1 1] Make Herders always rotate towards Player
  (if (`self.bRotateTowardsPlayer`)
    (`self.K2_SetActorRotation` (`KismetMathLibrary.MakeRotator` 0.0 0.0 (.yaw (`KismetMathLibrary.FindLookAtRotation` (`self.K2_GetActorLocation`) (`self.K2_GetActorLocation` (`GameplayStatics.GetPlayerCharacter` 0))))))))

(event `EnableStageTwo`
  ;[1 1 1] Called from Herder_BT in task: MoveToPoint
  (set `self.bStageOneComplete` true))

(fn `UserConstructionScript`)